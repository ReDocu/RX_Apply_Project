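; BP_InvenComponent is an inventory component that stores item data in a Slot array.
; AddItem and RemoveItem add and remove entries directly, with no capacity or duplicate checks.
; FindItem searches the array linearly by item name and returns whether a match exists.
; BeginPlay and Tick are disabled placeholders, so the component does work only when its functions are called.
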(event EventBeginPlay)

(event EventTick
  (params (DeltaSeconds :type Float%20%28single-precision%29)))

(fn AddItem
  (params (ItemData :type ST%20Item%20Type%20Structure))
  (Utilities|Array|Add (Variables|Default|GetSlot) ItemData))

(fn RemoveItem
  (params (ItemData :type ST%20Item%20Type%20Structure))
  (Utilities|Array|RemoveItem (Variables|Default|GetSlot) ItemData))

(fn FindItem
  (params (FindItem :type String))
  (for _array_element (Variables|Default|GetSlot)
    (if (Utilities|Enum|Equal(Enum) (.name _array_element) FindItem)
      (return true)))
  (return false))