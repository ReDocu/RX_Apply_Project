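; BP_Drawer is a grabbable drawer that slides along its forward axis as a motion controller moves.
; Its GrabComponent's grab and drop events toggle tracking and record the controller's starting location.
; While grabbed, Tick projects the controller's movement since the last frame onto the actor's forward vector and applies it as a teleporting local X offset.
; The graph applies no travel limits.
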(event OnGrabbed(GrabComponent)
  (Variables|Default|SetGrabLocation (Transformation|GetWorldLocation (Variables|/Game/VRTemplate/Blueprints/GrabComponent.GrabComponent_C|GetMotionControllerRef (Variables|Default|GetGrabComponent))))
  (Variables|Default|SetGrabbed true))

(event OnDropped(GrabComponent)
  (Variables|Default|SetGrabbed false))

(event EventTick
  (params (DeltaSeconds :type Float%20%28single-precision%29))
  (bind _grabcomponent (Variables|Default|GetGrabComponent))
  (bind _motioncontrollerref (Variables|/Game/VRTemplate/Blueprints/GrabComponent.GrabComponent_C|GetMotionControllerRef _grabcomponent))
  (bind _returnvalue (Transformation|GetWorldLocation _motioncontrollerref))
  (if (Variables|Default|GetGrabbed)
    (Transformation|AddActorLocalOffset (Math|Vector|MakeVector (Math|Vector|DotProduct (- _returnvalue (Variables|Default|GetGrabLocation)) (Transformation|GetActorForwardVector)) 0.0 0.0) false true)
    (Variables|Default|SetGrabLocation _returnvalue)))

(fn ConstructionScript)