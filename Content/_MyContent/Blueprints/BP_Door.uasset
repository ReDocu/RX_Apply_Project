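; BP_Door is a door actor that opens and closes according to whether its linked gimmicks are complete.
; On BeginPlay it binds to the quest-complete event of every gimmick in BPGimmickComponent.
; Each event rechecks whether all gimmicks are complete, then plays or reverses a timeline that yaws the door mesh up to 90 degrees.
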(event Custom|OpenDoor
  (bind _locationz (Timeline|DoorTimeLIne PlayFromStart)
    (:Update
      (Transformation|SetRelativeRotation (Variables|Default|GetSM_Door) (Math|Rotator|MakeRotator 0.0 0.0 (* _locationz 9e+01)) false false))))

(event Custom|CloseDoor
  (bind _locationz (Timeline|DoorTimeLIne ReverseFromEnd)
    (:Update
      (Transformation|SetRelativeRotation (Variables|Default|GetSM_Door) (Math|Rotator|MakeRotator 0.0 0.0 (* _locationz 9e+01)) false false))))

(event Custom|EventGimmickComplete
  (bind _isallcomplete (Default|IsAllGimmickComplete (Variables|Default|GetBP_GimmickComponent)))
  (if _isallcomplete
    (CallFunction|OpenDoor)
    (else
      (CallFunction|CloseDoor))))

(event EventBeginPlay
  (for _array_element (Variables|/Game/_MyContent/Blueprints/BP_GimmickComponent.BP_GimmickComponent_C|GetBP_Gimmicks (Variables|Default|GetBP_GimmickComponent))
    (EventDispatchers|BindEventtoQuestComplete _array_element (delegate Custom|EventGimmickComplete))))

(fn ConstructionScript)