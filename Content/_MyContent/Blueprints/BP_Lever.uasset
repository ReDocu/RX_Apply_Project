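; BP_Lever is a lever actor that can be grabbed with a motion controller, but its movement logic is unfinished.
; GrabComponent events set the Grabbed flag and, on grab, store the controller location and the lever mesh's relative pitch.
; Tick checks Grabbed but does nothing.
; An unconnected calculation projects current and initial grab vectors onto the actor's swing plane and takes their signed cross product about the right axis.
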(event OnGrabbed(GrabComponent)
  (Variables|Default|SetGrabLocation (Transformation|GetWorldLocation (Variables|/Game/VRTemplate/Blueprints/GrabComponent.GrabComponent_C|GetMotionControllerRef (Variables|Default|GetGrabComponent))))
  (Variables|Default|SetGrabRelativeRotationRotY (.pitch (Variables|/Script/Engine.SceneComponent|GetRelativeRotation (Variables|Default|GetSKM_Lever_SM_Lever1))))
  (Variables|Default|SetGrabbed true))

(event OnDropped(GrabComponent)
  (Variables|Default|SetGrabbed false))

(event EventTick
  (params (DeltaSeconds :type Float%20%28single-precision%29))
  (if (Variables|Default|GetGrabbed)
    _))

(fn ConstructionScript)