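; BP_Stage_1_1 is a pressure button gimmick, apparently for stage 1-1, that reports to a quest check when triggered.
; It caches the Button's world location at BeginPlay as the rest position.
; Any Box overlap plays a timeline that lerps the Button slightly downward and calls OnCheckQuest with true.
; Ending the overlap reverses the timeline to raise the Button, without sending a false quest check.
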(event OnComponentBeginOverlap(Box)
  (params (OverlappedComponent :type Primitive%20Component%20Object%20Reference) (OtherActor :type Actor%20Object%20Reference) (OtherComp :type Primitive%20Component%20Object%20Reference) (OtherBodyIndex :type Integer) (bFromSweep :type Boolean) (SweepResult :type Hit%20Result%20Structure%20%28by%20ref%29))
  (bind _initiallocation (Variables|Default|GetInitialLocation))
  (Utilities|FlowControl|Sequence
    (:then_0
      (bind _location (Timeline|ButtonTimeline Play)
        (:Update
          (Transformation|SetWorldLocation (Variables|Default|GetButton) (Math|Vector|Lerp(Vector) _initiallocation (- _initiallocation "0.000000,0.000000,3.000000") _location) false false))))
    (:then_1
      (CallFunction|OnCheckQuest true))))

(event OnComponentEndOverlap(Box)
  (params (OverlappedComponent :type Primitive%20Component%20Object%20Reference) (OtherActor :type Actor%20Object%20Reference) (OtherComp :type Primitive%20Component%20Object%20Reference) (OtherBodyIndex :type Integer))
  (bind _initiallocation (Variables|Default|GetInitialLocation))
  (bind _location (Timeline|ButtonTimeline Reverse)
    (:Update
      (Transformation|SetWorldLocation (Variables|Default|GetButton) (Math|Vector|Lerp(Vector) _initiallocation (- _initiallocation "0.000000,0.000000,3.000000") _location) false false))))

(event EventBeginPlay
  (Variables|Default|SetInitialLocation (Transformation|GetWorldLocation (Variables|Default|GetButton))))

(fn ConstructionScript
  (|CallParentFunction))