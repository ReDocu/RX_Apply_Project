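; BP_Gimmick_ItemCheck is a gimmick that checks whether the player holds the statue item and reports it to a quest check.
; On BeginPlay it binds CheckItem to the VR pawn's take-grab event.
; CheckItem searches the pawn's inventory component for BP_Statue by name and calls OnCheckQuest with true when found.
; It never reports a failed check.
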(event Custom|CheckItem
  (bind _returnvalue (Game|Player|GetPlayerPawn 0))
  (bind _returnvalue_2 (Actor|GetComponentbyClass _returnvalue "/Game/_MyContent/Blueprints/BP_InvenComponent.BP_InvenComponent_C"))
  (Utilities|IsValid _returnvalue_2
    (:Is%20Valid
      (bind _exist (Default|FindItem _returnvalue_2 "BP_Statue"))
      (if _exist
        (CallFunction|OnCheckQuest true)))))

(event EventBeginPlay
  (bind _asvrpawn (Utilities|Casting|CastToVRPawn (Game|Player|GetPlayerPawn 0)))
  (EventDispatchers|BindEventtoTakeGrab _asvrpawn (delegate Custom|CheckItem)))

(fn ConstructionScript
  (|CallParentFunction))