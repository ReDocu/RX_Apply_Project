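; BP_Gimmick_CheckPoint is a checkpoint gimmick that reports quest completion based on whether actors are inside its Box trigger.
; Begin and end overlaps add or remove valid actors in OverlapActors, then share one check on that list.
; The check calls OnCheckQuest with true while any actor remains, printing a debug success string, and false when empty.
; OnCheckQuest and the construction script only forward to the parent class.
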(event OnComponentBeginOverlap(Box)
  (params (OverlappedComponent :type Primitive%20Component%20Object%20Reference) (OtherActor :type Actor%20Object%20Reference) (OtherComp :type Primitive%20Component%20Object%20Reference) (OtherBodyIndex :type Integer) (bFromSweep :type Boolean) (SweepResult :type Hit%20Result%20Structure%20%28by%20ref%29))
  (bind _overlapactors (Variables|Default|GetOverlapActors))
  (Utilities|IsValid OtherActor
    (:Is%20Valid
      (Utilities|Array|Add _overlapactors OtherActor)
      (if (> (Utilities|Array|Length _overlapactors) 0)
        (CallFunction|OnCheckQuest true)
        (Development|PrintString "성공1")
        (else
          (CallFunction|OnCheckQuest false))))))

(event OnComponentEndOverlap(Box)
  (params (OverlappedComponent :type Primitive%20Component%20Object%20Reference) (OtherActor :type Actor%20Object%20Reference) (OtherComp :type Primitive%20Component%20Object%20Reference) (OtherBodyIndex :type Integer))
  (Utilities|IsValid OtherActor
    (:Is%20Valid
      (Utilities|Array|RemoveItem (Variables|Default|GetOverlapActors) OtherActor)
      (if (> (Utilities|Array|Length (Variables|Default|GetOverlapActors)) 0)
        (CallFunction|OnCheckQuest true)
        (Development|PrintString "성공1")
        (else
          (CallFunction|OnCheckQuest false))))))

(fn ConstructionScript
  (|CallParentFunction))

(fn OnCheckQuest
  (params (CheckComplete :type Boolean))
  (|CallParentFunction CheckComplete))