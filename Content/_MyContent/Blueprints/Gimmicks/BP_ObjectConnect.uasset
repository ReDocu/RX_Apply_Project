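; BP_ObjectConnect is a gimmick Blueprint that accepts a specific item, identified by MatchCheckItem, to progress a quest check.
; OnCheckItem shows the CheckUp indicator for a matching item while the gimmick is incomplete, and hides it for a mismatch.
; On a match, SetCheckItem calls OnCheckQuest, swaps CheckUp for the SMCornerFrame component and returns true.
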(fn ConstructionScript
  (|CallParentFunction))

(fn OnCheckItem
  (params (MatchingItem :type Grab%20Component%20Object%20Reference))
  (if (== (Variables|Default|GetMatchCheckItem) MatchingItem)
    (if (not (Variables|Default|GetIsComplete))
      (Rendering|SetVisibility (Variables|Default|GetCheckUp) true false))
    (else
      (Rendering|SetVisibility (Variables|Default|GetCheckUp) false false))))

(fn SetCheckItem
  (params (MatchingItem :type Grab%20Component%20Object%20Reference))
  (if (== (Variables|Default|GetMatchCheckItem) MatchingItem)
    (CallFunction|OnCheckQuest true)
    (Rendering|SetVisibility (Variables|Default|GetCheckUp) false false)
    (Rendering|SetVisibility (Variables|Default|GetSM_CornerFrame) true false)
    (return true)))